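; BP_Caja is a box ("caja") Blueprint that holds name, current health, maximum health and damage variables and prints them to the screen for debugging.
; BeginPlay joins the labeled Spanish values into a single string and shows it with Print String as colored, timed text.
; Tick, overlap and the construction script do nothing, and a leftover DeltaSeconds print is never executed.
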(event EventBeginPlay
  (Development|PrintString (Utilities|String|Append "Nombre: 
" (Variables|Default|Getnombre) " 
Vida Actual: 
" (Utilities|String|ToString(Float) (Variables|Default|Getvida)) " 
Vida Maxima: 
" (Utilities|String|ToString(Float) (Variables|Default|GetVidaMaxima)) " 
Daño: 
" (Utilities|String|ToString(Float) (Variables|Default|GetDaño))) true true "(R=0.438290,G=0.116117,B=1.000000,A=1.000000)" 15.0))

(event Collision|EventActorBeginOverlap
  (params (OtherActor :type Actor%20Object%20Reference)))

(event EventTick
  (params (DeltaSeconds :type Float%20%28single-precision%29)))

(fn ConstructionScript)